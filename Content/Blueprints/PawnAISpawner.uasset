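; Spawner actor that creates an AI pawn of CharacterToSpawn at its own transform and keeps it patrolling between two points.
; The construction script adds two box components at the relative locations Goal1 and Goal2.
; BeginPlay sends the pawn to the first box with AIMoveTo.
; Each box's overlap event checks for that spawned pawn and sends it to the opposite box with SimpleMoveToLocation, forming a loop without timers.
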(event OnComponentBeginOverlap(GoalBox1)
  (params (OtherActor :type Actor%20Object%20Reference) (OtherComp :type Primitive%20Component%20Object%20Reference) (OtherBodyIndex :type Integer) (bFromSweep :type Boolean) (SweepResult :type Hit%20Result%20Structure%20%28by%20ref%29))
  (bind _aspawn (Utilities|Casting|CastToPawn OtherActor))
  (if (== _aspawn (Variables|Default|GetPawnVariable))
    (AI|Navigation|SimpleMovetoLocation (Pawn|GetController _aspawn) (Transformation|GetWorldLocation (Variables|Default|GetGoalBox2)))))

(event OnComponentBeginOverlap(GoalBox2)
  (params (OtherActor :type Actor%20Object%20Reference) (OtherComp :type Primitive%20Component%20Object%20Reference) (OtherBodyIndex :type Integer) (bFromSweep :type Boolean) (SweepResult :type Hit%20Result%20Structure%20%28by%20ref%29))
  (bind _aspawn (Utilities|Casting|CastToPawn OtherActor))
  (if (== _aspawn (Variables|Default|GetPawnVariable))
    (AI|Navigation|SimpleMovetoLocation (Pawn|GetController _aspawn) (Transformation|GetWorldLocation (Variables|Default|GetGoalBox1)))))

(event EventBeginPlay
  (bind _returnvalue (Transformation|GetActorTransform))
  (Variables|Default|SetGoalBox1 (Variables|Default|GetGoalBox1))
  (bind _returnvalue_2 (AI|SpawnAIFromClass (Variables|Default|GetCharacterToSpawn) 0 (.location _returnvalue) (.rotation _returnvalue) false))
  (bind _output_get (Variables|Default|SetPawnVariable _returnvalue_2))
  (AI|AIMoveTo _output_get (Transformation|GetWorldLocation (Variables|Default|GetGoalBox1)) 0 5.0 false))

(event EventActorBeginOverlap
  (params (OtherActor :type Actor%20Object%20Reference)))

(fn ConstructionScript
  (bind _returnvalue (AddComponent|AddBoxComponent false (Math|Transform|MakeTransform (Variables|Default|GetGoal1) "0, 0, 0" "1,1,1")))
  (Variables|Default|SetGoalBox1 _returnvalue)
  (bind _returnvalue_2 (AddComponent|AddBoxComponent false (Math|Transform|MakeTransform (Variables|Default|GetGoal2) "0, 0, 0" "1,1,1")))
  (Variables|Default|SetGoalBox2 _returnvalue_2))